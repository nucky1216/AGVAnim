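; Scissor fork Blueprint for a scissor lifter that so far only visualizes linkage geometry in the editor, with no runtime logic.
; The Construction Script passes the relative Y/Z positions of Sphere2 and Sphere1 to CirclePoints as centers of two equal-radius circles.
; CirclePoints solves their intersections analytically and draws both circles.
; The script prints the result and marks intersections with debug points, using relative coordinates directly as world positions.
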(fn `CirclePoints`
  (params (Center1 :type "Vector2D Structure") (Center2 :type "Vector2D Structure") (R1 :type "Float (double-precision)") (R2 :type "Float (double-precision)"))
  (returns (Intersection1 :type "Vector2D Structure") (Intersection2 :type "Vector2D Structure") (Intersection :type Boolean))
  (locals (Distance :type "Float (double-precision)" :default 0.0) (a :type "Float (double-precision)") (h :type "Float (double-precision)" :default 0.0) (x3 :type "Float (double-precision)") (y3 :type "Float (double-precision)"))
  (bind _r1 (`local.R1`))
  (bind (_x _y) (`KismetMathLibrary.BreakVector2D` (`local.Center2`)))
  (bind (_x_2 _y_2) (`KismetMathLibrary.BreakVector2D` (`local.Center1`)))
  (bind (_x_3 _y_3) (`KismetMathLibrary.BreakVector2D` (`local.Center2`)))
  (bind (_x_4 _y_4) (`KismetMathLibrary.BreakVector2D` (`local.Center1`)))
  (bind _returnvalue (/ (* (- _x _x_4) (`local.h`)) (`local.Distance`)))
  (bind _returnvalue_2 (/ (* (- _y _y_4) (`local.h`)) (`local.Distance`)))
  (set `local.Distance` (`KismetMathLibrary.Distance2D` Center1 Center2))
  (if (or (> (`local.Distance`) (+ (`local.R1`) (`local.R2`))) (< (`local.Distance`) (`KismetMathLibrary.Abs` (- (`local.R1`) (`local.R2`)))))
    (return (0.0 0.0) (0.0 0.0) false)
    (else
      (`|ExecutionSequence`
        (:`then_0`
          (set `local.a` (/ (+ (- (`KismetMathLibrary.Square` (`local.R1`)) (`KismetMathLibrary.Square` (`local.R2`))) (`KismetMathLibrary.Square` (`local.Distance`))) (* (`local.Distance`) 2.0))))
        (:`then_1`
          (set `local.h` (`KismetMathLibrary.Sqrt` (`KismetMathLibrary.Abs` (- (`KismetMathLibrary.Square` (`local.R1`)) (`KismetMathLibrary.Square` (`local.a`)))))))
        (:`then_2`
          (set `local.x3` (+ _x_2 (/ (* (- _x_3 _x_2) (`local.a`)) (`local.Distance`)))))
        (:`then_3`
          (set `local.y3` (+ _y_2 (/ (* (- _y_3 _y_2) (`local.a`)) (`local.Distance`)))))
        (:`then_4`
          (`self.Debug DrawCircle` (`local.Center1`) _r1)
          (`self.Debug DrawCircle` (`local.Center2`) _r1))
        (:`then_5`
          (return (`KismetMathLibrary.MakeVector2D` (+ (`local.x3`) _returnvalue_2) (- (`local.y3`) _returnvalue)) (`KismetMathLibrary.MakeVector2D` (- (`local.x3`) _returnvalue_2) (+ (`local.y3`) _returnvalue)) true))))))

(fn `Debug DrawCircle`
  (params (Center :type "Vector2D Structure") (R :type "Float (double-precision)"))
  (bind (_x _y) (`KismetMathLibrary.BreakVector2D` Center))
  (`KismetSystemLibrary.DrawDebugCircle` (`KismetMathLibrary.MakeVector` 0.0 _x _y) R 30 (struct :`G` 1.0 :`B` 1.0 :`A` 1.0) 2.0 10.0 (0.0 1.0 0.0) (0.0 0.0 1.0) true))

(fn `UserConstructionScript`
  (bind _r1 (`self.R1`))
  (bind (_x _y _z) (`KismetMathLibrary.BreakVector3f` (`SceneComponent.RelativeLocation` (`self.Sphere1`))))
  (bind (_x_2 _y_2 _z_2) (`KismetMathLibrary.BreakVector3f` (`SceneComponent.RelativeLocation` (`self.Sphere2`))))
  (bind (_intersection1 _intersection2 _intersection) (`self.CirclePoints` (`KismetMathLibrary.MakeVector2D` _y_2 _z_2) (`KismetMathLibrary.MakeVector2D` _y _z) _r1 _r1))
  (`KismetSystemLibrary.PrintString` (`KismetStringLibrary.Concat_StrStr` (`KismetStringLibrary.Conv_Vector2dToString` _intersection1) "++" (`KismetStringLibrary.Conv_Vector2dToString` _intersection2) "-->" (`KismetStringLibrary.Conv_BoolToString` _intersection)))
  (if _intersection
    (bind (_x_3 _y_3) (`KismetMathLibrary.BreakVector2D` _intersection1))
    (`KismetSystemLibrary.DrawDebugPoint` (`KismetMathLibrary.MakeVector` 0.0 _x_3 _y_3) 20.0 (struct :`R` 1.0 :`A` 1.0) 2.0)
    (bind (_x_4 _y_4) (`KismetMathLibrary.BreakVector2D` _intersection2))
    (`KismetSystemLibrary.DrawDebugPoint` (`KismetMathLibrary.MakeVector` 0.0 _x_4 _y_4) 20.0 (struct :`R` 1.0 :`A` 1.0) 2.0)))