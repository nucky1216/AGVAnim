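; Carrier pawn that transports packages, exposing movement and handling steps while its own BeginPlay and Tick stay empty.
; AIMoveToTarget and MoveTo issue AI move requests; an unwired MoveBySpline ping-pongs along a spline and sets the look-ahead point used for turning.
; Drag, lift and rotate functions advance one increment per call and return completion, moving packages between carrier and work-area slot.
; SetState and GetState expose an on-package flag.
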(event `self.ReceiveBeginPlay`)

(event `self.ReceiveTick`
  (params (DeltaSeconds :type "Float (single-precision)")))

(event `AIMoveToTarget`
  (params (Location :type "Vector Structure"))
  (bind _movementresult (`|AIMoveTo` self Location null 25.0)
    (:`then`
      (`DimensioBPLibrary.PrintLog` (`|GetEnumeratorNameAsString` _movementresult)))))

(fn `CheckNeedToRotate`
  (returns (RotateNow :type Boolean))
  (bind _returnvalue (`self.GetActorForwardVector`))
  (bind _returnvalue_2 (!= _returnvalue (`KismetMathLibrary.Normal` (- (`self.NextLocation`) (`self.K2_GetActorLocation`))) :`ErrorTolerance` 0.0001))
  (`|ExecutionSequence`
    (:`then_0`
      (if _returnvalue_2
        (set `self.CurForward` _returnvalue)))
    (:`then_1`
      (return _returnvalue_2))))

(fn `Drag Package`
  (params (Package :type "Actor Object Reference") (InverseProcess :type Boolean) (WorkArea :type "/Game/VO/AGV_Carrier/BP_AreaEtis Object Reference"))
  (returns (Finish :type Boolean))
  (locals (TargetLocation :type "Vector Structure"))
  (bind _returnvalue (`self.K2_GetActorLocation` Package))
  (set `local.TargetLocation` (select `bool` (`local.InverseProcess`) :`false` (+ (`self.K2_GetActorLocation`) (0.0 0.0 50.0)) :`true` (`/Game/VO/AGV_Carrier/BP_AreaEtis.GetPakTargetSlot` WorkArea)))
  (`self.K2_SetActorLocation` Package (+ (* (`KismetMathLibrary.Normal` (- (`local.TargetLocation`) _returnvalue)) (* (`self.Speed`) 1.0)) _returnvalue) false false)
  (return (<= (`KismetMathLibrary.Vector_Distance` (`self.K2_GetActorLocation` Package) (`local.TargetLocation`)) 10.0)))

(fn `GetState`
  (returns (OnPak :type Boolean))
  (return (`self.OnPakState`)))

(fn `Lift Package`
  (params (Package :type "Actor Object Reference") (Inverse :type Boolean))
  (returns (Finished :type Boolean))
  (bind _returnvalue (+ (`self.K2_GetActorLocation` Package) (* (`self.GetActorUpVector` Package) (* (`self.Speed`) (`KismetMathLibrary.SelectFloat` -1.0 1.0 Inverse)))))
  (bind _returnvalue_2 (`KismetMathLibrary.VSize` (* (- _returnvalue (`self.K2_GetActorLocation`)) (`self.GetActorUpVector`))))
  (`self.K2_SetActorLocation` Package _returnvalue false false)
  (return (select `bool` (`local.Inverse`) :`false` (>= _returnvalue_2 (`self.LiftHeight`)) :`true` (<= _returnvalue_2 (`self.UnLiftHeight`)))))

(fn `MoveBySpline`
  (bind _spline (`self.Spline`))
  (`|ExecutionSequence`
    (:`then_0`
      (if (>= (`self.M_Dist`) (`SplineComponent.GetSplineLength` _spline))
        (set `self.Inverse` true)))
    (:`then_1`
      (if (< (`self.M_Dist`) 0.0)
        (set `self.Inverse` false)))
    (:`then_2`
      (bind _output_get (set `self.M_Dist` (+ (`self.M_Dist`) (* (`self.Speed`) (`KismetMathLibrary.SelectFloat` -1.0 1.0 (`self.Inverse`))))))
      (`self.K2_SetActorLocation` (.location (`SplineComponent.GetTransformAtDistanceAlongSpline` _spline _output_get "World" false)))
      (set `self.NextLocation` (`SplineComponent.GetLocationAtDistanceAlongSpline` (`self.GetComponentByClass` (`self.Target`) "/Script/Engine.SplineComponent") (+ (`self.M_Dist`) (* (`self.Speed`) (`KismetMathLibrary.SelectFloat` -1.0 1.0 (`self.Inverse`)))) "World")))))

(fn `MoveTo`
  (`AIBlueprintHelperLibrary.SimpleMoveToLocation` (`AIBlueprintHelperLibrary.GetAIController` self) (`self.Goal`)))

(fn `RotateToForward`
  (returns (Finish :type Boolean))
  (bind _returnvalue (`self.K2_GetActorLocation`))
  (bind _output_get (set `self.RotLerp` (+ (`self.RotLerp`) (`self.RotStep`))))
  (`KismetSystemLibrary.DrawDebugPoint` (`self.NextLocation`) 20.0 (struct :`R` 0.554 :`A` 1.0) 0.005)
  (`self.K2_SetActorRotation` (`KismetMathLibrary.RLerp` (`KismetMathLibrary.FindLookAtRotation` _returnvalue (+ (* (`self.CurForward`) 200.0) _returnvalue)) (`KismetMathLibrary.FindLookAtRotation` _returnvalue (`self.NextLocation`)) _output_get true))
  (if (>= (`self.RotLerp`) 1.0)
    (set `self.RotLerp` 0.0)
    (return true)
    (else
      (return false))))

(fn `SetState`
  (params (On :type Boolean))
  (set `self.OnPakState` On))

(fn `UserConstructionScript`)