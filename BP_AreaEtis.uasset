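; BP_AreaEtis is a package area that carriers work at, as either a pickup (UpLoad) or a drop-off zone.
; Packages are added at the end and removed from the front, each change refreshing NeedWorker against a target count: empty for UpLoad, full slots otherwise.
; A carrier qualifies when work remains and its carrying state opposes UpLoad.
; Local slot offsets become world targets, and construction tints the plane by type.
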(fn `CheckAbleToWork`
  (params (Carrier :type "/Game/VO/AGV_Carrier/BP_Carrier Object Reference"))
  (returns (Able :type Boolean))
  (return (and (`self.NeedWorker`) (xor (`self.UpLoad`) (`/Game/VO/AGV_Carrier/BP_Carrier.OnPakState` Carrier)))))

(fn `CheckWorkFinished`
  (set `self.NeedWorker` (!= (`self.FinishNum`) (`KismetArrayLibrary.Array_Length` (`self.Packages`)))))

(fn `GetPakTargetSlot`
  (returns (Slot :type "Vector Structure"))
  (bind _slots (`self.Slots`))
  (bind _returnvalue (`KismetArrayLibrary.Array_Length` (`self.Packages`)))
  (if (> (`KismetArrayLibrary.Array_Length` _slots) _returnvalue)
    (return (`KismetMathLibrary.TransformLocation` (`self.GetTransform`) (`|GetArrayItem` _slots _returnvalue)))
    (else
      (return (0.0 0.0 0.0)))))

(fn `Pop Paks`
  (returns (Package :type "Actor Object Reference"))
  (locals (TempPak :type "Actor Object Reference"))
  (bind _packages (`self.Packages`))
  (set `local.TempPak` (`|GetArrayItem` _packages))
  (`KismetArrayLibrary.Array_Remove` _packages)
  (`self.CheckWorkFinished`)
  (return (`local.TempPak`)))

(fn `Push Paks`
  (params (`New Pak` :type "Actor Object Reference"))
  (returns (NewPak :type "Actor Object Reference"))
  (`KismetArrayLibrary.Array_Add` (`self.Packages`) `New Pak`)
  (`self.CheckWorkFinished`)
  (return `New Pak`))

(fn `SetFinishNum`
  (set `self.FinishNum` (`KismetMathLibrary.SelectInt` 0 (`KismetArrayLibrary.Array_Length` (`self.Slots`)) (`self.UpLoad`))))

(fn `SetPlaneMat`
  (params (NewParam :type "LinearColor Structure"))
  (`MeshComponent.SetVectorParameterValueOnMaterials` (`self.Plane`) "Color" (`KismetMathLibrary.Conv_LinearColorToVector` NewParam)))

(fn `TestLoc`
  (for _array_element (`self.Slots`)
    (`DimensioBPLibrary.PrintLog` (`KismetStringLibrary.Conv_VectorToString` (`KismetMathLibrary.TransformLocation` (`self.GetTransform`) _array_element)))))

(fn `TypeToColor`
  (`self.SetPlaneMat` (select `bool` (`self.UpLoad`) :`false` (struct :`R` 0.104 :`G` 0.025607 :`B` 0.020638 :`A` 1.0) :`true` (struct :`R` 0.028569 :`G` 0.117 :`B` 0.025407 :`A` 1.0) :!type "LinearColor Structure")))

(fn `UserConstructionScript`
  (`self.CheckWorkFinished`)
  (`self.TypeToColor`))