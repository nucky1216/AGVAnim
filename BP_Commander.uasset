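; BP_Commander is a commander actor that sends every BP_Carrier_2 in the level toward a shared target area.
; On BeginPlay it caches all carriers in an array.
; Its GoToTarget event picks a random reachable navigation point within a small radius of the Actor variable's location, logs it, and passes it to each carrier's AIMoveToTarget.
; A leftover FlipFlop branch is never triggered.
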(event `self.ReceiveBeginPlay`
  (bind _outactors (`GameplayStatics.GetAllActorsOfClass` "/Game/VO/AGV_Carrier/BP_Carrier_2.BP_Carrier_2_C"))
  (set `self.Out Actors` _outactors))

(event `GoToTarget`
  (bind _output_get (set `self.Random Location` (`NavigationSystemV1.K2_GetRandomReachablePointInRadius` (`self.K2_GetActorLocation` (`self.Actor`)) 50.0 null null)))
  (`DimensioBPLibrary.PrintLog` (`KismetStringLibrary.Conv_VectorToString` _output_get))
  (for _array_element (`self.Out Actors`)
    (`/Game/VO/AGV_Carrier/BP_Carrier_2.AIMoveToTarget` _array_element (`self.Random Location`))))

(fn `UserConstructionScript`)